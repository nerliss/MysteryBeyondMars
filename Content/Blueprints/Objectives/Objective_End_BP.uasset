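; Objective_End_BP is a trigger actor that completes a specific player objective when the player enters its box.
; On overlap, it checks that the player character's current objective matches its own Objective, then prefixes it with "Completed:".
; It plays a completion sound, finds the HUD widget by class to fire its objective update event, then destroys itself.
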(event `self.Box.OnComponentBeginOverlap`
  (params (OverlappedComponent :type "PrimitiveComponent Object Reference") (OtherActor :type "Actor Object Reference") (OtherComp :type "PrimitiveComponent Object Reference") (OtherBodyIndex :type Integer) (bFromSweep :type Boolean) (SweepResult :type "HitResult Structure (by ref)"))
  (bind _objective (`self.Objective`))
  (bind _asplayer_character_bp (cast `/Game/Blueprints/Player/PlayerCharacter_BP` OtherActor))
  (if (== (`/Game/Blueprints/Player/PlayerCharacter_BP.CurrentObjective` _asplayer_character_bp) _objective)
    (set `/Game/Blueprints/Player/PlayerCharacter_BP.CurrentObjective` (`KismetStringLibrary.Concat_StrStr` "Completed: " _objective) _asplayer_character_bp)
    (`GameplayStatics.PlaySound2D` "/Game/Assets/Sounds/Objectives/A_UI_Objective_Complete.A_UI_Objective_Complete" 1.0 1.0 0.0 null null)
    ;[1 1 1] Used as Cast to widget class
    (bind _foundwidgets (`WidgetBlueprintLibrary.GetAllWidgetsOfClass` "/Game/UI/HUD_WBP.HUD_WBP_C"))
    (`/Game/UI/Objective/Objective_WBP.EventOnObjectUpdated` (`/Game/UI/HUD_WBP.Objective_WBP` (`|GetArrayItem` _foundwidgets)))
    (`self.K2_DestroyActor`)))

(fn `UserConstructionScript`)