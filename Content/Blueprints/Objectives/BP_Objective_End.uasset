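; Objective end trigger actor that clears a completed objective from play when the player character overlaps it.
; On overlap, it checks that the ProjectNCharacter's CurrentObjective is non-empty and equals its own Objective prefixed with "Completed:".
; On a match, it finds WBP_HUD, fires EventOnObjectUpdated on its ObjectiveWBP and destroys itself.
; The overlap logic stays in Blueprint because the widgets it calls are Blueprint-based.
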(event `self.ReceiveActorBeginOverlap`
  (params (OtherActor :type "Actor Object Reference"))
  ;[1 1 1] This is still called in BP because all of WBPs are written via Blueprints
  (bind _asproject_ncharacter (cast `ProjectNCharacter` OtherActor))
  (bind _currentobjective (`ProjectNCharacter.CurrentObjective` _asproject_ncharacter))
  (if (and (not (`KismetStringLibrary.IsEmpty` _currentobjective)) (== _currentobjective (`KismetStringLibrary.Concat_StrStr` "Completed: " (`self.Objective`))))
    ;;[1 1 1] Used as Cast to widget class
    (bind _foundwidgets (`WidgetBlueprintLibrary.GetAllWidgetsOfClass` "/Game/UI/WBP_HUD.WBP_HUD_C"))
    (`/Game/UI/Objective/WBP_Objective.EventOnObjectUpdated` (`/Game/UI/WBP_HUD.Objective_WBP` (`|GetArrayItem` _foundwidgets)))
    (`self.K2_DestroyActor`)))

(fn `UserConstructionScript`)