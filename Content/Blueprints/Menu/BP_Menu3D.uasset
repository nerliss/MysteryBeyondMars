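; BP_Menu3D is a 3D menu actor that hosts a widget and hands the view to linked menu actors.
; It starts hidden and binds to its WBP_3D_Base widget's transition event, whose index selects from LinkedMenus.
; A transition swaps collision, blends the camera to the next menu, then swaps visibility after a delay shorter than the blend.
; Timeline-driven opacity fade nodes are unconnected and never run.
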(event `self.ReceiveBeginPlay`
  (`|ExecutionSequence`
    (:`then_0`
      (`self.SetActorHiddenInGame` true))
    (:`then_1`
      ;[1 1 1] Bind transit event then call it in different menus depending on their indices
      (bind _aswbp_3d_base (cast `/Game/UI/Menu/Main/WBP_3D_Base` (`WidgetComponent.GetUserWidgetObject` (`self.Widget`))))
      (add `/Game/UI/Menu/Main/WBP_3D_Base.TransitionToLinkedMenu` _aswbp_3d_base (delegate `OnTransitionBetweenMenus`)))))

(event `OnTransitionBetweenMenus`
  (params (MenuIndex :type Integer))
  (bind _linkedmenus (`self.LinkedMenus`))
  ;[1 1 1] Bind transit event then call it in different menus depending on their indices
  (if (`KismetArrayLibrary.Array_IsValidIndex` _linkedmenus MenuIndex)
    (`self.TransitToNextWidget` (`|GetArrayItem` _linkedmenus MenuIndex))))

(event `TransitToNextWidget`
  (params (NewMenu :type "/Game/Blueprints/Menu/BP_Menu3D Object Reference"))
  ;[1 1 1] Transit to next widget
  (`self.SetActorEnableCollision` false)
  (`self.SetActorEnableCollision` NewMenu true)
  (`PlayerController.SetViewTargetWithBlend` (`GameplayStatics.GetPlayerController` 0) NewMenu 1.5 "VTBlend_Linear" 0.0 false)
  (`KismetSystemLibrary.Delay` 1.0)
  (`self.SetActorHiddenInGame` NewMenu false)
  (`self.SetActorHiddenInGame` true))

(fn `UserConstructionScript`)