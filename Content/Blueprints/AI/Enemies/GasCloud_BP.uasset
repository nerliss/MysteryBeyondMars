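; GasCloud_BP is a roaming gas cloud enemy that kills the player on proximity.
; It loops through a short delay and an AI move to a random reachable point around itself, retrying on failure, while an attached ambient sound plays.
; Tick compares player and cloud locations with a per-axis tolerance instead of using overlap, calling the player's Death once through a DoOnce.
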(event `self.ReceiveBeginPlay`
  ;[1 1 1] Advanced move to
  (`|ExecutionSequence`
    (:`then_0`
      (`KismetSystemLibrary.Delay` 2.0 :!label _label)
      (`|AIMoveTo` self (`NavigationSystemV1.K2_GetRandomReachablePointInRadius` (`self.K2_GetActorLocation`) 5000.0 null null) null
        (:`OnSuccess`
          (goto _label))
        (:`OnFail`
          (goto _label))))
    (:`then_1`
      (`GameplayStatics.SpawnSoundAttached` "/Game/Assets/Sounds/GasCloudAmbLoop_Cue.GasCloudAmbLoop_Cue" (`self.CapsuleComponent`) "None" (0.0 0.0 0.0) (struct) "KeepRelativeOffset" false 1.0 1.0 0.0 null null))))

(event `self.ReceiveTick`
  (params (DeltaSeconds :type "Float (single-precision)"))
  ;[1 1 1] Test decision - kill player if they are in +-300 range of gas cloud location
  (`parent.ReceiveTick` DeltaSeconds)
  (bind _asplayer_character_bp (cast `/Game/Blueprints/Player/PlayerCharacter_BP` (`GameplayStatics.GetPlayerPawn` 0)))
  (if (== (`self.K2_GetActorLocation` _asplayer_character_bp) (`self.K2_GetActorLocation`) :`ErrorTolerance` 300.0)
    (`/Engine/EditorBlueprintResources/StandardMacros.DoOnce` false
      (:`Completed`
        (`/Game/Blueprints/Player/PlayerCharacter_BP.Death` _asplayer_character_bp)))))

(fn `UserConstructionScript`
  (`parent.UserConstructionScript`))