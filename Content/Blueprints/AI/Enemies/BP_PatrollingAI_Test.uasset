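; Test patrolling enemy AI that walks four locations and kills the player on capsule overlap while its seeing flag is set.
; BeginPlay runs the patrol loop, restarting after completion or failure, or branches to a move with fade-in chase music.
; Tick fades the music out and resets its once-gate after a delayed recheck finds no sighting.
; The sight-flag update logic is disconnected, and the chase move has no target.
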(event `self.ReceiveBeginPlay`
  (bind (_locations_location1 _locations_location2 _locations_location3 _locations_location4) (break `/Game/Blueprints/AI/Enemies/SAIPatrolPoints` (`self.Locations`)))
  (bind _returnvalue (`AddComponent|NODE_AddAudioComponent-0`))
  (bind _output_get (set `self.ChaseMusic` _returnvalue))
  (`AudioComponent.Stop` _output_get)
  ;[1 1 1] Patrol
  (if (not (`self.isSeeingTheEnemy`)) :!label _label
    (`|AIMoveTo` self _locations_location1 null 20.0
      (:`OnSuccess`
        (`|AIMoveTo` self _locations_location2 null 20.0
          (:`OnSuccess`
            (`|AIMoveTo` self _locations_location3 null 20.0
              (:`OnSuccess`
                (`|AIMoveTo` self _locations_location4 null 20.0
                  (:`OnSuccess`
                    _)
                  (:`OnFail`
                    _)))
              (:`OnFail`
                _)))
          (:`OnFail`
            _)))
      (:`OnFail`
        _))
    (`KismetSystemLibrary.Delay` 1.0)
    (goto _label)
    (else
      (`|AIMoveTo` self (0.0 0.0 0.0) null 20.0
        (:`then`
          (`/Engine/EditorBlueprintResources/StandardMacros.DoOnce` false :!label _label_2
            (:`Completed`
              (`AudioComponent.FadeIn` (`self.ChaseMusic`) 2.0 1.0 0.5 "Linear"))))))))

(event `self.ReceiveTick`
  (params (DeltaSeconds :type "Float (single-precision)"))
  (bind _returnvalue (not (`self.isSeeingTheEnemy`)))
  (if _returnvalue
    (`KismetSystemLibrary.Delay` 0.4)
    (if _returnvalue
      (`AudioComponent.FadeOut` (`self.ChaseMusic`) 3.0 0.0 "Linear")
      (goto _label_2 :!via `Reset`))))

(event `self.CapsuleComponent.OnComponentBeginOverlap`
  (params (OverlappedComponent :type "PrimitiveComponent Object Reference") (OtherActor :type "Actor Object Reference") (OtherComp :type "PrimitiveComponent Object Reference") (OtherBodyIndex :type Integer) (bFromSweep :type Boolean) (SweepResult :type "HitResult Structure (by ref)"))
  ;[1 1 1] Kill player upon reaching
  (bind _asbp_player_character (cast `/Game/Blueprints/Player/BP_PlayerCharacter` OtherActor))
  (if (`self.isSeeingTheEnemy`)
    (`/Game/Blueprints/Player/BP_PlayerCharacter.Death` _asbp_player_character)))

(fn `UserConstructionScript`
  (`parent.UserConstructionScript`))