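; Player character Blueprint with debug-style key bindings: K plays a test montage, and P triggers Death, which ragdolls the mesh and detaches the controller.
; E and Tick share a camera-forward line trace with debug drawing, so it runs every frame.
; Any hit BaseEnemyBP tagged BaseEnemy has its name printed and IsAlive cleared.
; The construction script caps frame rate through a console command.
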(event `Key|K`
  (params (Key :type "Key Structure"))
  (:`Pressed`
    (`|PlayMontage` (`self.Mesh`) "/Game/Assets/Characters/Mannequin/Animations/TestAnim_Montage.TestAnim_Montage")))

(event `Death`
  (`PrimitiveComponent.SetCollisionEnabled` (`self.CapsuleComponent`) "NoCollision")
  (`PrimitiveComponent.SetSimulatePhysics` (`self.Mesh`) true)
  (`self.DetachFromControllerPendingDestroy`)
  (`KismetSystemLibrary.Delay` 1.0))

(event `Key|P`
  (params (Key :type "Key Structure"))
  (:`Pressed`
    (`self.Death`)))

(event `Key|E`
  (params (Key :type "Key Structure"))
  (bind _followcamera (`self.FollowCamera`))
  (bind _returnvalue (`SceneComponent.K2_GetComponentLocation` _followcamera))
  (:`Pressed`
    (bind (_outhit _returnvalue_2) (`KismetSystemLibrary.LineTraceSingle` :`Start` _returnvalue :`End` (+ _returnvalue (* (`KismetMathLibrary.GetForwardVector` (`SceneComponent.K2_GetComponentRotation` _followcamera)) (`KismetMathLibrary.Conv_DoubleToVector` 500.0))) :`TraceChannel` "TraceTypeQuery2" :`bTraceComplex` true :`DrawDebugType` "ForDuration" :!label _label))
    (if _returnvalue_2
      (bind _output_get (set `self.OutHitTarget` (`.HitActor` (`GameplayStatics.BreakHitResult` _outhit))))
      (if (`self.ActorHasTag` _output_get "BaseEnemy")
        (bind _asbase_enemy_bp (cast `/Game/Blueprints/Enemies/BaseEnemyBP` _output_get)
          (:`then`
            (`KismetSystemLibrary.PrintString` (`KismetTextLibrary.Conv_TextToString` (`/Game/Blueprints/Enemies/BaseEnemyBP.Name` _asbase_enemy_bp)))
            (set `/Game/Blueprints/Enemies/BaseEnemyBP.isAlive` false _asbase_enemy_bp))
          (:`CastFailed`
            (`KismetSystemLibrary.PrintString` "Failed to get the name of out hit")))))))

(event `self.ReceiveTick`
  (params (DeltaSeconds :type "Float (single-precision)"))
  (goto _label))

(fn `UserConstructionScript`
  (`KismetSystemLibrary.ExecuteConsoleCommand` "t.maxfps 70" null))