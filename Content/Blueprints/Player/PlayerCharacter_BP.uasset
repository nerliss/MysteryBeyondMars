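; Player character Blueprint handling interaction prompts, map toggling, objective checks, prone movement, wall running and death.
; Tick lazily creates the HUD, then line-traces from the camera to show names and prompts for GetName_BPI actors.
; A temporary horizontal wall run uses overlaps with tagged walls and a timeline to suspend gravity and push forward while Space is held.
; Death ragdolls the mesh, then saves a pose snapshot; construction caps FPS.
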(event `Death`
  (bind _mesh (`self.Mesh`))
  ;[1 1 1] Death
  (set `self.bDead` true)
  (`PrimitiveComponent.SetCollisionEnabled` (`self.CapsuleComponent`) "NoCollision")
  (`PrimitiveComponent.SetSimulatePhysics` _mesh true)
  (`self.DetachFromControllerPendingDestroy`)
  (`KismetSystemLibrary.Delay` 2.0)
  (`AnimInstance.SavePoseSnapshot` (`SkeletalMeshComponent.GetAnimInstance` _mesh) "Ragdoll")
  (`PrimitiveComponent.SetSimulatePhysics` _mesh false))

(event `Key|E`
  (params (Key :type "Key Structure"))
  (:`Pressed`
    (`KismetSystemLibrary.PrintString` "E is pressed in player class")))

(event `Key|P`
  (params (Key :type "Key Structure"))
  ;[1 1 1] Test: call function death
  (:`Pressed`
    (`self.Death`)))

(event `self.ReceiveTick`
  (params (DeltaSeconds :type "Float (single-precision)"))
  ;[1 1 1] Validate hud
  (`self.HUDRef`
    (:`then`
      (`self.GetObjectName`))
    (:`else`
      (`self.CreateHUD`))))

(event `self.ReceiveBeginPlay`
  ;[1 1 1] Begin play
  (`MovementComponent.SetPlaneConstraintEnabled` (`self.CharacterMovement`) true))

(event `GetObjectName`
  (bind _followcamera (`self.FollowCamera`))
  (bind _hudref (`self.HUDRef`))
  (bind _returnvalue (`SceneComponent.K2_GetComponentLocation` _followcamera))
  (bind _actionprompt_wbp (`/Game/UI/HUD_WBP.ActionPrompt_WBP` _hudref))
  ;[1 1 1] Linetrace - returns name of an object and interaction prompt
  (bind (_outhit _returnvalue_2) (`KismetSystemLibrary.LineTraceSingle` _returnvalue (+ _returnvalue (* (`KismetMathLibrary.GetForwardVector` (`SceneComponent.K2_GetComponentRotation` _followcamera)) (`KismetMathLibrary.Conv_DoubleToVector` 200.0))) "TraceTypeQuery2" true))
  (if _returnvalue_2
    (bind _output_get (set `self.HitTarget` (`.HitActor` (`GameplayStatics.BreakHitResult` _outhit))))
    (if (`KismetSystemLibrary.DoesImplementInterface` _output_get "/Game/Blueprints/Interfaces/GetName_BPI.GetName_BPI_C")
      (bind _name (message `/Game/Blueprints/Interfaces/GetName_BPI.GetName` _output_get))
      (set `/Game/UI/HUD_WBP.Name` _name _hudref)
      (`Widget.SetVisibility` _actionprompt_wbp "Visible")
      (`Widget.SetIsEnabled` _actionprompt_wbp true)
      (else
        (set `/Game/UI/HUD_WBP.Name` "" _hudref :!label _label)
        (`Widget.SetVisibility` _actionprompt_wbp "Hidden")
        (`Widget.SetIsEnabled` _actionprompt_wbp false)))
    (else
      (set `self.HitComponent` null)
      (goto _label))))

(event `CreateHUD`
  ;[1 1 1] Create main hud
  (bind _returnvalue (`|CreateWidget` "/Game/UI/HUD_WBP.HUD_WBP_C"))
  (bind _output_get (set `self.HUDRef` _returnvalue))
  (`UserWidget.AddToViewport` _output_get 0)
  ;[1 1 1] Hide player mesh on both minimap and big map
  (`SceneCaptureComponent.HideComponent` (`self.Minimap`) (`self.Mesh`))
  (`SceneCaptureComponent.HideComponent` (`self.Bigmap`) (`self.Mesh`)))

(event `InputAction|Crouch`
  (params (Key :type "Key Structure"))
  ;[1 1 1] Legacy: done in C++
  ;;[1 1 1] Crouching
)

(event `InputAction|OpenMap`
  (params (Key :type "Key Structure"))
  (bind _minimapcamera (`self.MinimapCamera`))
  (bind _hudref (`self.HUDRef`))
  (bind _bigmap_wbp (`/Game/UI/HUD_WBP.Bigmap_WBP` _hudref))
  (bind _minimap_wbp (`/Game/UI/HUD_WBP.Minimap_WBP` _hudref))
  ;[1 1 1] Open big map
  (:`Pressed`
    (`/Engine/EditorBlueprintResources/StandardMacros.FlipFlop`
      (:`A`
        (`Widget.SetIsEnabled` _bigmap_wbp true)
        (`Widget.SetVisibility` _bigmap_wbp "Visible")
        (`Widget.SetIsEnabled` _minimap_wbp false)
        (`Widget.SetVisibility` _minimap_wbp "Hidden")
        (set `SpringArmComponent.TargetArmLength` 10000.0 _minimapcamera))
      (:`B`
        (`Widget.SetIsEnabled` _bigmap_wbp false)
        (`Widget.SetVisibility` _bigmap_wbp "Hidden")
        (`Widget.SetIsEnabled` _minimap_wbp true)
        (`Widget.SetVisibility` _minimap_wbp "Visible")
        (set `SpringArmComponent.TargetArmLength` 2500.0 _minimapcamera)))))

(event `InputAction|CheckCurrentObjective`
  (params (Key :type "Key Structure"))
  (bind _objective_wbp (`/Game/UI/HUD_WBP.Objective_WBP` (`self.HUDRef`)))
  (bind _fadeinout (`/Game/UI/Objective/Objective_WBP.FadeInOut` _objective_wbp))
  (bind _bcancheckcurrentobjective (`/Game/UI/Objective/Objective_WBP.bCanCheckCurrentObjective` _objective_wbp))
  ;[1 1 1] Check current objective
  (:`Pressed`
    (if _bcancheckcurrentobjective
      (`UserWidget.PlayAnimation` _objective_wbp _fadeinout 0.0 1 "Forward" 1.0 false)))
  (:`Released`
    (if _bcancheckcurrentobjective
      (`UserWidget.PlayAnimation` _objective_wbp _fadeinout 0.0 1 "Reverse" 1.0 false))))

(event `InputAction|Prone`
  (params (Key :type "Key Structure"))
  (bind _charactermovement (`self.CharacterMovement`))
  ;[1 1 1] Prone
  (:`Pressed`
    (if (`self.bProning`)
      (set `self.bProning` false)
      (set `self.bGettingUp` true)
      (`KismetSystemLibrary.Delay` 1.3)
      (set `CharacterMovementComponent.MaxWalkSpeed` 600.0 _charactermovement)
      (else
        (set `self.bProning` true)
        (set `self.bGettingUp` false)
        (set `CharacterMovementComponent.MaxWalkSpeed` 160.0 _charactermovement)))))

(event `self.OnLanded`
  (params (Hit :type "HitResult Structure (by ref)"))
  ;[1 1 1] Temp solution. TODO: rewrite wall run on C++
  (bind _output_get (set `self.JumpMaxCount` 2)))

(event `self.WallDetection.OnComponentBeginOverlap`
  (params (OverlappedComponent :type "PrimitiveComponent Object Reference") (OtherActor :type "Actor Object Reference") (OtherComp :type "PrimitiveComponent Object Reference") (OtherBodyIndex :type Integer) (bFromSweep :type Boolean) (SweepResult :type "HitResult Structure (by ref)"))
  (bind _charactermovement (`self.CharacterMovement`))
  (bind _charactermovement_2 (`self.CharacterMovement`))
  ;[1 1 1] Horizontal wall run
  (`|ExecutionSequence`
    (:`then_0`
      ;[1 1 1] Temp solution. TODO: rewrite wall run on C++
      (bind _result (`/Engine/EditorBlueprintResources/StandardMacros.IncrementInt` (stale `self.OnLanded` _output_get))
        (:`  `
          (bind _output_get (set `self.JumpMaxCount` _result))
          (`KismetSystemLibrary.PrintString` (`KismetStringLibrary.Conv_IntToString` _output_get)))))
    (:`then_1`
      (set `self.PlayerCurrentDirection` (`SceneComponent.GetForwardVector` (`self.Mesh`)))
      (if (and (`self.ActorHasTag` OtherActor "RunnableWall") (`NavMovementComponent.IsFalling` (`self.CharacterMovement`)))
        (set `self.bOnWall` true)
        (`Timeline|WallRun` :!label _label_2
          (:`Update`
            (if (> (`PlayerController.GetInputKeyTimeDown` (`GameplayStatics.GetPlayerController` 0) "SpaceBar") 0.0)
              (if (`self.bOnWall`)
                (set `CharacterMovementComponent.GravityScale` 0.0 _charactermovement_2)
                (`MovementComponent.SetPlaneConstraintNormal` _charactermovement_2 (0.0 0.0 0.0)) ; Z is used by default
                (`CharacterMovementComponent.AddForce` _charactermovement_2 (* (`self.PlayerCurrentDirection`) (`KismetMathLibrary.Conv_DoubleToVector` 1000.0)))
                (else
                  (set `CharacterMovementComponent.GravityScale` 1.0 _charactermovement :!label _label_3)
                  (`MovementComponent.SetPlaneConstraintNormal` _charactermovement (0.0 0.0 0.0))
                  (set `self.bOnWall` false)))
              (else
                (goto _label_3)))))))))

(event `self.WallDetection.OnComponentEndOverlap`
  (params (OverlappedComponent :type "PrimitiveComponent Object Reference") (OtherActor :type "Actor Object Reference") (OtherComp :type "PrimitiveComponent Object Reference") (OtherBodyIndex :type Integer))
  ;[1 1 1] Horizontal wall run
  (`|ExecutionSequence`
    (:`then_0`
      (goto _label_2 :!via `Stop`))
    (:`then_1`
      (if (`self.ActorHasTag` OtherActor "RunnableWall")
        (goto _label_3)))))

(fn `UserConstructionScript`
  (`KismetSystemLibrary.ExecuteConsoleCommand` "t.maxfps 70" null))