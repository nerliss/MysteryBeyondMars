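; Door Blueprint that opens and closes when it receives an Interact event.
; BeginPlay creates a player for the DoorOpenClose level sequence.
; Each Interact toggles the IsOpen flag and plays that sequence forward to open or in reverse to close, so one animation serves both directions.
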(event `self.ReceiveBeginPlay`
  (bind (_outactor _returnvalue) (`LevelSequencePlayer.CreateLevelSequencePlayer` "/Game/Blueprints/Items/DoorOpenClose.DoorOpenClose")))

(event `/Game/Blueprints/Interfaces/Interact_BPI.Interact`
  (if (not (`self.isOpen`))
    (`MovieSceneSequencePlayer.Play` (stale `self.ReceiveBeginPlay` _returnvalue))
    (set `self.isOpen` true)
    (else
      (`MovieSceneSequencePlayer.PlayReverse` (stale `self.ReceiveBeginPlay` _returnvalue))
      (set `self.isOpen` false))))

(fn `UserConstructionScript`
  (`parent.UserConstructionScript`))