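; BP_Vocabulary is an interactable pickup that grants the player the vocabulary, turning giant's note text into human language.
; Interact sets HasVocabulary on BP_PlayerCharacter, prints a message, plays a pickup sound and destroys the actor.
; It also flags the first BP_GiantsNote found in the level and calls its ApplyNewDynamicMaterial, so no tick polling is needed.
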(event `/Game/Blueprints/Interfaces/BPI_Interact.Interact`
  (bind _asplayer_character_bp (cast `/Game/Blueprints/Player/BP_PlayerCharacter` (`GameplayStatics.GetPlayerPawn` 0)))
  (set `/Game/Blueprints/Player/BP_PlayerCharacter.hasVocabulary` true _asplayer_character_bp)
  (`KismetSystemLibrary.PrintString` "You've found the vocabulary!" true true (struct :`R` 0.20927 :`G` 1.0 :`B` 0.047743 :`A` 1.0) 4.0)
  ;[1 1 1] Set PlayerHasVocabulary in GiantsNote_BP class
  (bind _asbp_giants_note (castclass `/Game/Blueprints/Items/BP_GiantsNote` "/Game/Blueprints/Items/BP_GiantsNote.BP_GiantsNote_C"))
  (bind _outactors (`GameplayStatics.GetAllActorsOfClass` _asbp_giants_note))
  (bind _output (`|GetArrayItem` _outactors))
  (set `/Game/Blueprints/Items/BP_GiantsNote.PlayerHasVocabulary` true _output)
  ;[1 1 1] Changes language of giant's notes to human. Called here so there will be no need to use event tick
  (`/Game/Blueprints/Items/BP_GiantsNote.ApplyNewDynamicMaterial` _output)
  (`GameplayStatics.PlaySoundAtLocation` "/Game/Assets/Sounds/A_Vocabulary_PickUp.A_Vocabulary_PickUp" (`self.K2_GetActorLocation`) (struct) 1.0 1.0 0.0 null null null)
  (`self.K2_DestroyActor`))

(fn `IsInteractable`
  (returns (isInteractable :type Boolean))
  (return true))

(fn `UserConstructionScript`
  (`parent.UserConstructionScript`))