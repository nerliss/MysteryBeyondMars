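; Interactable hinged door that toggles between open and closed each time Interact fires.
; The Open flag selects whether the DoorRotation timeline plays from the start or reverses from the end, and its Angle track sets the Hinge component's relative yaw.
; Both calls restart from an endpoint, so interacting mid-swing snaps the door.
; Disconnected player-facing dot product and Direction nodes do not affect the swing.
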(event `/Game/Blueprints/Interfaces/BPI_Interact.Interact`
  (if (not (`self.bOpen`))
    (set `self.bOpen` true)
    (bind (_direction _angle) (`Timeline|DoorRotation` :!via `PlayFromStart` :!label _label)
      (:`Update`
        (`SceneComponent.K2_SetRelativeRotation` (`self.Hinge`) (`KismetMathLibrary.MakeRotator` 0.0 0.0 _angle) false false)))
    (else
      (set `self.bOpen` false)
      (goto _label :!via `ReverseFromEnd`))))

(fn `UserConstructionScript`
  (`parent.UserConstructionScript`))