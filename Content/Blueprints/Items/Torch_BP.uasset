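; Torch item that the player can pick up and carry, with a looping or one-shot fire sound cue attached to its handle on BeginPlay.
; It always reports itself as interactable.
; On Interact, if the player is neither holding a torch nor swimming, it snaps onto the player's item hold point, disables handle collision and sets the player's holding-torch flag.
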(event `self.ReceiveBeginPlay`
  (`GameplayStatics.SpawnSoundAttached` "/Game/Assets/Sounds/Ambient/Fire/Fire_Torch_Cue.Fire_Torch_Cue" (`self.Handle`) "None" (0.0 0.0 0.0) (struct) "KeepRelativeOffset" true 0.2 1.0 0.0 null null))

(event `/Game/Blueprints/Interfaces/Interact_BPI.Interact`
  (bind _asplayer_character_bp (cast `/Game/Blueprints/Player/PlayerCharacter_BP` (`GameplayStatics.GetPlayerPawn` 0)))
  (if (not (`/Game/Blueprints/Player/PlayerCharacter_BP.isHoldingTorch` _asplayer_character_bp))
    (if (not (`/Game/Blueprints/Player/PlayerCharacter_BP.isSwimming` _asplayer_character_bp))
      (`self.K2_AttachToComponent` (`/Game/Blueprints/Player/PlayerCharacter_BP.ItemHoldScene` _asplayer_character_bp) "None" "SnapToTarget" "SnapToTarget" "SnapToTarget")
      (`PrimitiveComponent.SetCollisionEnabled` (`self.Handle`) "NoCollision")
      (set `/Game/Blueprints/Player/PlayerCharacter_BP.isHoldingTorch` true _asplayer_character_bp))))

(fn `IsInteractable`
  (returns (isInteractable :type Boolean))
  (return true))

(fn `UserConstructionScript`
  (`parent.UserConstructionScript`))