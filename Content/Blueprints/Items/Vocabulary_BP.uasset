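; Vocabulary_BP is an interactable pickup that lets the player read the giant's note in human language.
; On interact it sets HasVocabulary on the player, prints a confirmation, plays a pickup sound and destroys itself.
; It also flags the first GiantsNote_BP actor found and calls its ApplyNewDynamicMaterial to switch the language, avoiding a Tick check.
; Only that first note instance is updated.
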(event `/Game/Blueprints/Interfaces/Interact_BPI.Interact`
  (bind _asplayer_character_bp (cast `/Game/Blueprints/Player/PlayerCharacter_BP` (`GameplayStatics.GetPlayerPawn` 0)))
  (set `/Game/Blueprints/Player/PlayerCharacter_BP.hasVocabulary` true _asplayer_character_bp)
  (`KismetSystemLibrary.PrintString` "You've found the vocabulary!" true true (struct :`R` 0.20927 :`G` 1.0 :`B` 0.047743 :`A` 1.0) 4.0)
  ;[1 1 1] Set PlayerHasVocabulary in GiantsNote_BP class
  (bind _asgiants_note_bp (castclass `/Game/Blueprints/Items/GiantsNote_BP` "/Game/Blueprints/Items/GiantsNote_BP.GiantsNote_BP_C"))
  (bind _outactors (`GameplayStatics.GetAllActorsOfClass` _asgiants_note_bp))
  (bind _output (`|GetArrayItem` _outactors))
  (set `/Game/Blueprints/Items/GiantsNote_BP.PlayerHasVocabulary` true _output)
  ;[1 1 1] Changes language of giant's notes to human. Called here so there will be no need to use event tick
  (`/Game/Blueprints/Items/GiantsNote_BP.ApplyNewDynamicMaterial` _output)
  (`GameplayStatics.PlaySoundAtLocation` "/Game/Assets/Sounds/A_Vocabulary_PickUp.A_Vocabulary_PickUp" (`self.K2_GetActorLocation`) (struct) 1.0 1.0 0.0 null null null)
  (`self.K2_DestroyActor`))

(fn `IsInteractable`
  (returns (isInteractable :type Boolean))
  (return true))

(fn `UserConstructionScript`
  (`parent.UserConstructionScript`))