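; BP_Note is an interactable paper note that the player picks up to read and puts down again.
; Interact toggles the player's IsHoldingNote flag, showing or removing Note_WBP, pausing or unpausing the game, and playing a paper sound on pickup.
; Tick re-reads that flag from the player to stay in sync.
; The construction script sets a dynamic material texture by note Number, so one class covers several notes.
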(event `self.ReceiveBeginPlay`
  ;[1 1 1] Create material ref
  (set `self.MaterialReference` (`PrimitiveComponent.GetMaterial` (`self.Note`) 0))
  (bind _asplayer_character_bp (cast `/Game/Blueprints/Player/BP_PlayerCharacter` (`GameplayStatics.GetPlayerPawn` 0)))
  (set `self.PlayerReference` _asplayer_character_bp)
  (`self.EnableInput` (`GameplayStatics.GetPlayerController` 0)))

(event `self.ReceiveTick`
  (params (DeltaSeconds :type "Float (single-precision)"))
  ;[1 1 1] Calling isHoldingNote from player object again so we wouldn't need to press interaction key once again while looking at note after we close NoteWidget by pause button
  (set `self.IsPlayerHoldingNote` (`/Game/Blueprints/Player/BP_PlayerCharacter.isHoldingNote` (`self.PlayerReference`))))

(event `/Game/Blueprints/Interfaces/BPI_Interact.Interact`
  (bind _playerreference (`self.PlayerReference`))
  (if (not (`/Game/Blueprints/Player/BP_PlayerCharacter.isInPauseMenu` (`self.PlayerReference`)))
    (if (not (`self.IsPlayerHoldingNote`))
      ;[1 1 1] Take the note
      (bind _output_get (set `/Game/Blueprints/Player/BP_PlayerCharacter.isHoldingNote` true _playerreference))
      (set `self.IsPlayerHoldingNote` _output_get)
      (bind _returnvalue (`|CreateWidget` "/Game/UI/Notes/Note_WBP.Note_WBP_C"))
      (bind _output_get_2 (set `self.NoteWidgetReference` _returnvalue))
      (`UserWidget.AddToViewport` _output_get_2 0)
      (`GameplayStatics.SpawnSound2D` (select `int` (`KismetMathLibrary.RandomInteger` 2) :`0` "/Game/Assets/Sounds/A_Paper_01.A_Paper_01" :`1` "/Game/Assets/Sounds/A_Paper_02.A_Paper_02" :`2` "/Game/Assets/Sounds/A_Paper_03.A_Paper_03" :!type "SoundBase Object Reference") 1.0 1.0 0.0 null)
      (`GameplayStatics.SetGamePaused` true)
      (else
        ;[1 1 1] Put the note down
        (bind _output_get_3 (set `/Game/Blueprints/Player/BP_PlayerCharacter.isHoldingNote` false _playerreference))
        (set `self.IsPlayerHoldingNote` _output_get_3)
        (`Widget.RemoveFromParent` (`self.NoteWidgetReference`))
        (`GameplayStatics.SetGamePaused` false)))))

(event `Key|One`
  (params (Key :type "Key Structure"))
  ;[1 1 1] Deprecated
)

(fn `IsInteractable`
  (returns (isInteractable :type Boolean))
  (return true))

(fn `UserConstructionScript`
  (`parent.UserConstructionScript`)
  (set `self.OriginalTransform` (`self.GetTransform`))
  ;[1 1 1] Create dynamic material instance - changes content of the note depending on its number. I did this so there wont be any need to create multiple note classes
  (bind _returnvalue (`PrimitiveComponent.CreateDynamicMaterialInstance` (`self.Note`) 0 "/Game/Assets/Materials/Notes/MI_Note.MI_Note" "NoteDynamicMaterial"))
  (`MaterialInstanceDynamic.SetTextureParameterValue` _returnvalue "TextureParam" (select `int` (`self.Number`) :`0` "/Game/Assets/Materials/Notes/T_NoteTest_01.T_NoteTest_01" :`1` "/Game/Assets/Materials/Notes/T_NoteTest_02.T_NoteTest_02" :`2` "/Game/Assets/Materials/Notes/T_NoteTest_03.T_NoteTest_03" :!type "Texture Object Reference")))