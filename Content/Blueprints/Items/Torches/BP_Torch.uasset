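; BP_Torch is an interactable torch item that the player can pick up and carry, with a fire sound attached to its handle.
; On interact, it snaps to the player character's ItemHoldScene, provided the player is neither already holding a torch nor in water.
; Pickup also disables handle collision, sets the player's IsHoldingTorch flag, enables shadow casting on the handle and flammable part, and plays a pickup sound.
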(event `self.ReceiveBeginPlay`
  (`GameplayStatics.SpawnSoundAttached` "/Game/Assets/Sounds/Ambient/Fire/A_Fire_Torch_Cue.A_Fire_Torch_Cue" (`self.Handle`) "None" (0.0 0.0 0.0) (struct) "KeepRelativeOffset" true 0.2 1.0 0.0 null null))

(event `/Game/Blueprints/Interfaces/BPI_Interact.Interact`
  (bind _asbp_player_character (cast `/Game/Blueprints/Player/BP_PlayerCharacter` (`GameplayStatics.GetPlayerPawn` 0)))
  (if (not (`/Game/Blueprints/Player/BP_PlayerCharacter.isHoldingTorch` _asbp_player_character))
    (if (not (`ProjectNCharacter.bInWater` _asbp_player_character))
      (`self.K2_AttachToComponent` (`/Game/Blueprints/Player/BP_PlayerCharacter.ItemHoldScene` _asbp_player_character) "None" "SnapToTarget" "SnapToTarget" "SnapToTarget")
      (`PrimitiveComponent.SetCollisionEnabled` (`self.Handle`) "NoCollision")
      (set `/Game/Blueprints/Player/BP_PlayerCharacter.isHoldingTorch` true _asbp_player_character)
      (`PrimitiveComponent.SetCastShadow` (`self.FlammablePart`) true)
      (`PrimitiveComponent.SetCastShadow` (`self.Handle`) true)
      (`GameplayStatics.PlaySoundAtLocation` "/Game/Assets/Sounds/Torch/A_Torch_PickUp.A_Torch_PickUp" (`self.K2_GetActorLocation`) (struct) 0.7 1.0 0.0 null null null))))

(fn `IsInteractable`
  (returns (isInteractable :type Boolean))
  (return true))

(fn `UserConstructionScript`
  (`parent.UserConstructionScript`))