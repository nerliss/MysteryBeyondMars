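; BP_TorchExtinguished is an extinguished torch item that the player cannot interact with.
; It returns false from IsInteractable, leaves the Interact event empty and runs the parent construction script.
; A disconnected, unused pickup chain remains in the event graph, which would snap the torch to the player's ItemHoldScene, disable handle collision and set IsHoldingTorch.
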(event `/Game/Blueprints/Interfaces/BPI_Interact.Interact`)

(fn `IsInteractable`
  (returns (isInteractable :type Boolean))
  (return false))

(fn `UserConstructionScript`
  (`parent.UserConstructionScript`))