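; BP_Torch is an interactable torch item that the player can pick up and hold.
; It starts an attached fire sound on its handle at BeginPlay and always reports itself as interactable.
; On Interact, if the player character is neither holding a torch nor in water, it snaps onto the character's ItemHoldScene, disables handle collision and sets IsHoldingTorch on the character.
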(event `self.ReceiveBeginPlay`
  (`GameplayStatics.SpawnSoundAttached` "/Game/Assets/Sounds/Ambient/Fire/A_Fire_Torch_Cue.A_Fire_Torch_Cue" (`self.Handle`) "None" (0.0 0.0 0.0) (struct) "KeepRelativeOffset" true 0.2 1.0 0.0 null null))

(event `/Game/Blueprints/Interfaces/BPI_Interact.Interact`
  (bind _asplayer_character_bp (cast `/Game/Blueprints/Player/BP_PlayerCharacter` (`GameplayStatics.GetPlayerPawn` 0)))
  (if (not (`/Game/Blueprints/Player/BP_PlayerCharacter.isHoldingTorch` _asplayer_character_bp))
    (if (not (`ProjectNCharacter.bInWater` _asplayer_character_bp))
      (`self.K2_AttachToComponent` (`/Game/Blueprints/Player/BP_PlayerCharacter.ItemHoldScene` _asplayer_character_bp) "None" "SnapToTarget" "SnapToTarget" "SnapToTarget")
      (`PrimitiveComponent.SetCollisionEnabled` (`self.Handle`) "NoCollision")
      (set `/Game/Blueprints/Player/BP_PlayerCharacter.isHoldingTorch` true _asplayer_character_bp))))

(fn `IsInteractable`
  (returns (isInteractable :type Boolean))
  (return true))

(fn `UserConstructionScript`
  (`parent.UserConstructionScript`))