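; BP_GiantsNote is a note prop whose displayed text depends on its number and whether the player has the vocabulary.
; Construction creates a dynamic material instance and picks the page texture, using Giant variants for some numbers without vocabulary, so one class covers several notes.
; ApplyNewDynamicMaterial repeats that choice when BP_Vocabulary is picked up.
; IsInteractable returns false and Interact is empty, leaving the pick-up widget, sound and pause logic disconnected.
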(event `ApplyNewDynamicMaterial`
  (bind _dynamicmaterialinstancereference (`self.DynamicMaterialInstanceReference`))
  ;[1 1 1] Called in BP_Vocabulary upon taking it up
  (if (`self.PlayerHasVocabulary`)
    (`MaterialInstanceDynamic.SetTextureParameterValue` _dynamicmaterialinstancereference "TextureParam" (select `int` (`self.Number`) :`0` "/Game/Assets/Materials/Notes/Textures/T_NoteTest_04.T_NoteTest_04" :`1` "/Game/Assets/Materials/Notes/Textures/T_NoteTest_02.T_NoteTest_02" :`2` "/Game/Assets/Materials/Notes/Textures/T_NoteTest_03.T_NoteTest_03" :`3` null :`4` null :`5` "/Game/Assets/Materials/Notes/Textures/T_NoteTest_05.T_NoteTest_05" :!type "Texture Object Reference"))
    (else
      (`MaterialInstanceDynamic.SetTextureParameterValue` _dynamicmaterialinstancereference "TextureParam" (select `int` (`self.Number`) :`0` "/Game/Assets/Materials/Notes/Textures/T_NoteTest_Giant_04.T_NoteTest_Giant_04" :`1` "/Game/Assets/Materials/Notes/Textures/T_NoteTest_02.T_NoteTest_02" :`2` "/Game/Assets/Materials/Notes/Textures/T_NoteTest_03.T_NoteTest_03" :`3` null :`4` null :`5` "/Game/Assets/Materials/Notes/Textures/T_NoteTest_Giant_05.T_NoteTest_Giant_05" :!type "Texture Object Reference")))))

(event `self.ReceiveBeginPlay`
  ;[1 1 1] Create material ref
  (set `self.MaterialReference` (`PrimitiveComponent.GetMaterial` (`self.Note`) 0)))

(event `/Game/Blueprints/Interfaces/BPI_Interact.Interact`)

(fn `IsInteractable`
  (returns (isInteractable :type Boolean))
  (return false))

(fn `UserConstructionScript`
  (bind _number (`self.Number`))
  (`parent.UserConstructionScript`)
  ;[1 1 1] Create dynamic material instance - changes content of the note depending on its number and whether player has vocabulary or not. I did this so there wont be any need to create multiple note classes
  (bind _returnvalue (`PrimitiveComponent.CreateDynamicMaterialInstance` (`self.Note`) 0 "/Game/Assets/Materials/Notes/Materials_World/MI_Note.MI_Note" "None"))
  (bind _output_get (set `self.DynamicMaterialInstanceReference` _returnvalue))
  (if (`self.PlayerHasVocabulary`)
    (`MaterialInstanceDynamic.SetTextureParameterValue` _output_get "TextureParam" (select `int` _number :`0` "/Game/Assets/Materials/Notes/Textures/T_NoteTest_04.T_NoteTest_04" :`1` "/Game/Assets/Materials/Notes/Textures/T_NoteTest_02.T_NoteTest_02" :`2` "/Game/Assets/Materials/Notes/Textures/T_NoteTest_03.T_NoteTest_03" :`3` null :`4` null :`5` "/Game/Assets/Materials/Notes/Textures/T_NoteTest_05.T_NoteTest_05" :!type "Texture Object Reference"))
    (else
      (`MaterialInstanceDynamic.SetTextureParameterValue` _output_get "TextureParam" (select `int` _number :`0` "/Game/Assets/Materials/Notes/Textures/T_NoteTest_Giant_04.T_NoteTest_Giant_04" :`1` "/Game/Assets/Materials/Notes/Textures/T_NoteTest_02.T_NoteTest_02" :`2` "/Game/Assets/Materials/Notes/Textures/T_NoteTest_03.T_NoteTest_03" :`3` null :`4` null :`5` "/Game/Assets/Materials/Notes/Textures/T_NoteTest_Giant_05.T_NoteTest_Giant_05" :!type "Texture Object Reference")))))