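; Interactive dresser actor whose drawers the player slides open and closed with the E key.
; It enables its own input, then line-traces WorldDynamic objects from the player's follow camera and treats any hit Movable static mesh component as a drawer.
; The drawer's relative X decides open or close, and timelines lerp it a fixed distance with a sound.
; A CanOpen flag blocks input until the slide finishes.
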(event `self.ReceiveBeginPlay`
  (`self.EnableInput` (`GameplayStatics.GetPlayerController` 0))
  (bind _asplayer_character_bp (cast `/Game/Blueprints/Player/PlayerCharacter_BP` (`GameplayStatics.GetPlayerCharacter` 0)))
  (set `self.PlayerReference` _asplayer_character_bp)
  (`SceneComponent.SetMobility` (`self.dark-wood-dresser-with-fully-modelled-drawers3_SONGESAND_dresser`) "Static"))

(event `Key|E`
  (params (Key :type "Key Structure"))
  (bind _returnvalue (`self.K2_GetActorLocation`))
  (bind _playerreference (`self.PlayerReference`))
  (bind _staticmeshref (`self.StaticMeshRef`))
  (bind _staticmeshref_2 (`self.StaticMeshRef`))
  (bind _followcamera (`ProjectNCharacter.FollowCamera` _playerreference))
  (bind (_relativelocation_x _relativelocation_y _relativelocation_z) (`KismetMathLibrary.BreakVector` (`SceneComponent.RelativeLocation` _staticmeshref_2)))
  (bind (_relativelocation_x_2 _relativelocation_y_2 _relativelocation_z_2) (`KismetMathLibrary.BreakVector` (`SceneComponent.RelativeLocation` _staticmeshref_2)))
  (bind _returnvalue_2 (`SceneComponent.K2_GetComponentLocation` _followcamera))
  ;[1 1 1] Open\close drawers
  (:`Pressed`
    (if (`self.bCanOpen`)
      (bind (_outhit _returnvalue_3) (`KismetSystemLibrary.LineTraceSingleForObjects` _returnvalue_2 (+ _returnvalue_2 (* (`SceneComponent.GetForwardVector` _followcamera) (`KismetMathLibrary.Conv_DoubleToVector` 500.0))) (`|MakeArray` "ObjectTypeQuery2" :!type "EObjectTypeQuery Enum") true (`|MakeArray` _playerreference :!type "Actor Object Reference") "ForDuration" false))
      (if _returnvalue_3
        (bind _asstatic_mesh_component (cast `StaticMeshComponent` (`.HitComponent` (`GameplayStatics.BreakHitResult` _outhit)))
          (:`then`
            (if (`|EnumEquality` (`SceneComponent.Mobility` _asstatic_mesh_component) "Movable")
              (bind _output_get (set `self.StaticMeshRef` _asstatic_mesh_component))
              (set `self.bCanOpen` false)
              (bind _relativelocation_x_3 (`KismetMathLibrary.BreakVector` (`SceneComponent.RelativeLocation` _output_get)))
              (if (<= _relativelocation_x_3 25.0)
                (`GameplayStatics.PlaySoundAtLocation` "/Game/Assets/Sounds/Dresser/dresser_open.dresser_open" _returnvalue (struct) 1.0 1.0 0.0 null null null)
                (set `self.EndLocation` (`KismetMathLibrary.MakeVector` (+ _relativelocation_x_2 30.0) _relativelocation_y_2 _relativelocation_z_2))
                (set `self.StartLocation` (`KismetMathLibrary.MakeVector` _relativelocation_x_2 _relativelocation_y_2 _relativelocation_z_2))
                (bind (_direction _opendrawer) (`Timeline|OpenDrawer` :!via `PlayFromStart`)
                  (:`Update`
                    (`SceneComponent.K2_SetRelativeLocation` _staticmeshref (`KismetMathLibrary.VLerp` (`self.StartLocation`) (`self.EndLocation`) _opendrawer) false false))
                  (:`Finished`
                    (set `self.bCanOpen` true)))
                (else
                  (`GameplayStatics.PlaySoundAtLocation` "/Game/Assets/Sounds/Dresser/dresser_close.dresser_close" _returnvalue (struct) 1.0 1.0 0.0 null null null)
                  (set `self.EndLocation` (`KismetMathLibrary.MakeVector` (- _relativelocation_x 30.0) _relativelocation_y _relativelocation_z))
                  (set `self.StartLocation` (`KismetMathLibrary.MakeVector` _relativelocation_x _relativelocation_y _relativelocation_z))
                  (bind (_direction_2 _opendrawer_2) (`Timeline|CloseDrawer` :!via `PlayFromStart`)
                    (:`Update`
                      (`SceneComponent.K2_SetRelativeLocation` _staticmeshref (`KismetMathLibrary.VLerp` (`self.StartLocation`) (`self.EndLocation`) _opendrawer_2) false false))
                    (:`Finished`
                      (set `self.bCanOpen` true)))))))
          (:`CastFailed`
            (`KismetSystemLibrary.PrintString` "Poshel naxyi")))
        (else
          (`KismetSystemLibrary.PrintString` "No Hit Target or Hit Target doesn't have WorldDynamic Object Type"))))))

(fn `UserConstructionScript`
  (`parent.UserConstructionScript`))