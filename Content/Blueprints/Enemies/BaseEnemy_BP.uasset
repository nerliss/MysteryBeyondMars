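; Base enemy pawn that wanders at random while alive and ragdolls on death.
; BeginPlay starts a delayed AI move to a random reachable point nearby, repeating only on success.
; Death clears IsAlive, disables capsule collision, simulates mesh physics and detaches the controller.
; Pawn sensing is an empty hook with disconnected leftover logic, and the construction script sets a global frame-rate cap via console command.
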(event `Death`
  (set `self.isAlive` false)
  (`PrimitiveComponent.SetCollisionEnabled` (`self.CapsuleComponent`) "NoCollision")
  (`PrimitiveComponent.SetSimulatePhysics` (`self.Mesh`) true)
  (`self.DetachFromControllerPendingDestroy`))

(event `self.ReceiveBeginPlay`
  ;[1 1 1] Advanced move to
  (if (`self.isAlive`) :!label _label
    (`KismetSystemLibrary.Delay` 2.0)
    (`|AIMoveTo` self (`NavigationSystemV1.K2_GetRandomReachablePointInRadius` (`self.K2_GetActorLocation`) 5000.0 null null) null
      (:`OnSuccess`
        (goto _label)))))

(event `self.PawnSensing.OnSeePawn`
  (params (Pawn :type "Pawn Object Reference")))

(fn `GetName`
  (returns (Name :type Text))
  (return (`self.Name`)))

(fn `UserConstructionScript`
  (`KismetSystemLibrary.ExecuteConsoleCommand` "t.maxfps 70" null))